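; BP_Gene is a clickable actor that opens the gene menu.
; On BeginPlay it casts the game mode to ShipGM and caches the reference.
; When clicked while the game mode's GeneActive flag is set, it shows the game mode's GeneMenu widget and collapses the HUD.
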(event `self.ReceiveBeginPlay`
  (bind _asship_gm (cast `/Game/Me-Made/ShipGM` (`GameplayStatics.GetGameMode`)))
  (set `self.GM` _asship_gm))

(event `self.ReceiveActorOnClicked`
  (params (ButtonPressed :type "Key Structure"))
  (bind _gm (`self.GM`))
  (if (`/Game/Me-Made/ShipGM.GeneActive` _gm)
    (`Widget.SetVisibility` (`/Game/Me-Made/ShipGM.GeneMenu` _gm) "Visible")
    (`Widget.SetVisibility` (`/Game/Me-Made/ShipGM.HUD` _gm) "Collapsed")))

(fn `UserConstructionScript`)